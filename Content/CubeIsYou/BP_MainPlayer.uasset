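; BP_MainPlayer is the player input Blueprint for CubeIsYou, turning arrow keys into grid-style movement.
; On BeginPlay it caches the Cube_Inst game instance, shows the UI_CubeIsYou widget and enables the mouse cursor.
; Each arrow press sets a world-axis step and calls Move on every Cube, Cone, Sphere and Cylinder actor in turn.
; Input is ignored once the game is won, and a short delay on CanMove throttles repeated moves.
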(event `self.ReceiveBeginPlay`
  (bind _ascube_inst (cast `/Game/CubeIsYou/Cube_Inst` (`GameplayStatics.GetGameInstance`)))
  (set `self.As Cube Inst` _ascube_inst)
  (bind _returnvalue (`|CreateWidget` "/Game/CubeIsYou/UI_CubeIsYou.UI_CubeIsYou_C"))
  (bind _output_get (set `self.UI_Ref` _returnvalue))
  (`UserWidget.AddToViewport` _output_get 0)
  (set `PlayerController.bShowMouseCursor` true (`GameplayStatics.GetPlayerController` 0)))

(event `Key|Right`
  (params (Key :type "Key Structure"))
  (:`Pressed`
    (if (and (`self.CanMove`) (not (`/Game/CubeIsYou/Cube_Inst.Won?` (`self.As Cube Inst`))))
      (set `self.CanMove` false)
      (set `self.Direction` (0.0 100.0 0.0))
      (bind _outactors (`GameplayStatics.GetAllActorsOfClass` "/Game/CubeIsYou/BP_Cube.BP_Cube_C" :!label _label))
      (for _array_element _outactors
        (bind _asbp_cube (cast `/Game/CubeIsYou/BP_Cube` _array_element))
        (`/Game/CubeIsYou/BP_Cube.Move` _asbp_cube (`self.Direction`)))
      (bind _outactors_2 (`GameplayStatics.GetAllActorsOfClass` "/Game/CubeIsYou/BP_Cone.BP_Cone_C"))
      (for _array_element_2 _outactors_2
        (bind _asbp_cone (cast `/Game/CubeIsYou/BP_Cone` _array_element_2))
        (`/Game/CubeIsYou/BP_Cone.Move` _asbp_cone (`self.Direction`)))
      (bind _outactors_3 (`GameplayStatics.GetAllActorsOfClass` "/Game/CubeIsYou/BP_Sphere.BP_Sphere_C"))
      (for _array_element_3 _outactors_3
        (bind _asbp_sphere (cast `/Game/CubeIsYou/BP_Sphere` _array_element_3))
        (`/Game/CubeIsYou/BP_Sphere.Move` _asbp_sphere (`self.Direction`)))
      (bind _outactors_4 (`GameplayStatics.GetAllActorsOfClass` "/Game/CubeIsYou/BP_Cylinder.BP_Cylinder_C"))
      (for _array_element_4 _outactors_4
        (bind _asbp_cylinder (cast `/Game/CubeIsYou/BP_Cylinder` _array_element_4))
        (`/Game/CubeIsYou/BP_Cylinder.Move` _asbp_cylinder (`self.Direction`)))
      (`KismetSystemLibrary.Delay` 0.1)
      (set `self.CanMove` true))))

(event `Key|Up`
  (params (Key :type "Key Structure"))
  (:`Pressed`
    (if (and (`self.CanMove`) (not (`/Game/CubeIsYou/Cube_Inst.Won?` (`self.As Cube Inst`))))
      (set `self.CanMove` false)
      (set `self.Direction` (100.0 0.0 0.0))
      (goto _label))))

(event `Key|Left`
  (params (Key :type "Key Structure"))
  (:`Pressed`
    (if (and (`self.CanMove`) (not (`/Game/CubeIsYou/Cube_Inst.Won?` (`self.As Cube Inst`))))
      (set `self.CanMove` false)
      (set `self.Direction` (0.0 -100.0 0.0))
      (goto _label))))

(event `Key|Down`
  (params (Key :type "Key Structure"))
  (:`Pressed`
    (if (and (`self.CanMove`) (not (`/Game/CubeIsYou/Cube_Inst.Won?` (`self.As Cube Inst`))))
      (set `self.CanMove` false)
      (set `self.Direction` (-100.0 0.0 0.0))
      (goto _label))))

(fn `UserConstructionScript`)