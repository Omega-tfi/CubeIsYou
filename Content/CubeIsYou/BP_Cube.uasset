(event `CheckSink`
  (params (Type :type Integer) (Ref :type "Actor Object Reference"))
  (bind _as_cube_inst (`self.As Cube Inst`))
  (if (!= (`/Game/CubeIsYou/Cube_Inst.IsCubeSink` _as_cube_inst) (`|GetArrayItem` (`|MakeArray` false (`/Game/CubeIsYou/Cube_Inst.IsCubeSink` _as_cube_inst) (`/Game/CubeIsYou/Cube_Inst.IsConeSink?` _as_cube_inst) (`/Game/CubeIsYou/Cube_Inst.IsSphereSink?` _as_cube_inst) (`/Game/CubeIsYou/Cube_Inst.IsCylinderSink?` _as_cube_inst)) Type))
    (`self.K2_DestroyActor` Ref)
    (`self.K2_DestroyActor`)))

(event `CheckParticle`
  (`SceneComponent.SetHiddenInGame` (`self.Niagara`) (not (`/Game/CubeIsYou/Cube_Inst.IsCubeWin?` (`self.As Cube Inst`))) false))

(event `CheckWin`
  (params (Type :type Integer))
  (bind _as_cube_inst (`self.As Cube Inst`))
  (bind _as_cube_inst_2 (`self.As Cube Inst`))
  (bind _as_cube_inst_3 (`self.As Cube Inst`))
  (if (`/Game/CubeIsYou/Cube_Inst.IsCubeYou?` _as_cube_inst_2)
    (if (`|GetArrayItem` (`|MakeArray` false (`/Game/CubeIsYou/Cube_Inst.IsCubeWin?` _as_cube_inst) (`/Game/CubeIsYou/Cube_Inst.IsConeWin?` _as_cube_inst) (`/Game/CubeIsYou/Cube_Inst.IsSphereWin?` _as_cube_inst) (`/Game/CubeIsYou/Cube_Inst.IsCylinderWin?` _as_cube_inst)) Type)
      (bind _returnvalue (`|CreateWidget` "/Game/CubeIsYou/UI_Win.UI_Win_C" :!label _label))
      (`UserWidget.AddToViewport` _returnvalue 0)
      (set `/Game/CubeIsYou/Cube_Inst.Won?` true (`self.As Cube Inst`)))
    (elif (`/Game/CubeIsYou/Cube_Inst.IsCubeWin?` _as_cube_inst_2)
      (if (`|GetArrayItem` (`|MakeArray` false (`/Game/CubeIsYou/Cube_Inst.IsCubeYou?` _as_cube_inst_3) (`/Game/CubeIsYou/Cube_Inst.IsConeYou?` _as_cube_inst_3) (`/Game/CubeIsYou/Cube_Inst.IsSphereYou?` _as_cube_inst_3) (`/Game/CubeIsYou/Cube_Inst.IsCylinderYou?` _as_cube_inst_3)) Type)
        (goto _label)))))

(event `Check Collision`
  (`self.CheckParticle`)
  (if (not (`/Game/CubeIsYou/Cube_Inst.Won?` (`self.As Cube Inst`)))
    (for _array_element (`self.GetOverlappingActors` null)
      (bind _asbp_cube (cast `/Game/CubeIsYou/BP_Cube` _array_element)
        (:`then`
          (`self.CheckSink` 2 _asbp_cube)
          (`KismetSystemLibrary.DelayUntilNextTick`)
          (`self.CheckWin` 1))
        (:`CastFailed`
          (bind _asbp_cone (cast `/Game/CubeIsYou/BP_Cone` _array_element)
            (:`then`
              (`self.CheckSink` 2 _asbp_cone)
              (`KismetSystemLibrary.DelayUntilNextTick`)
              (`self.CheckWin` 2))
            (:`CastFailed`
              (bind _asbp_sphere (cast `/Game/CubeIsYou/BP_Sphere` _array_element)
                (:`then`
                  (`self.CheckSink` 3 _asbp_sphere)
                  (`KismetSystemLibrary.DelayUntilNextTick`)
                  (`self.CheckWin` 3))
                (:`CastFailed`
                  (bind _asbp_cylinder (cast `/Game/CubeIsYou/BP_Cylinder` _array_element))
                  (`self.CheckSink` 4 _asbp_cylinder)
                  (`KismetSystemLibrary.DelayUntilNextTick`)
                  (`self.CheckWin` 4))))))))))

(event `self.ReceiveBeginPlay`
  (bind _ascube_inst (cast `/Game/CubeIsYou/Cube_Inst` (`GameplayStatics.GetGameInstance`)))
  (set `self.As Cube Inst` _ascube_inst)
  (`KismetSystemLibrary.K2_SetTimerDelegate` (delegate `Check Collision`) 0.1 true))

(event `Move`
  (params (Direction :type "Vector Structure"))
  (if (`/Game/CubeIsYou/Cube_Inst.IsCubeYou?` (`self.As Cube Inst`))
    (set `self.Position` (`self.K2_GetActorLocation`))
    (bind (_direction _newtrack_0) (`Timeline|Timeline` :!via `PlayFromStart`)
      (:`Update`
        (`self.K2_SetActorLocation` (+ (* _newtrack_0 Direction) (`self.Position`)))))))

(fn `UserConstructionScript`)